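; BP_PodCharacter is the player-input side of the pod, relaying weapon controls to a separate BP_Pod actor.
; On BeginPlay it spawns BP_Pod at the world origin with itself as owner, stores the reference and calls Init on it.
; Press and release of the Fire Minigun and Fire Canon inputs call the pod's matching start and stop fire functions.
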(event EventBeginPlay
  (bind _returnvalue (Game|SpawnActorfromClass "/Game/Pod/BP_Pod.BP_Pod_C" (Math|Transform|MakeTransform "0, 0, 0") "AdjustIfPossibleButAlwaysSpawn" "OverrideRootScale" self 0))
  (Variables|Default|SetPod _returnvalue)
  (Default|Init _returnvalue))

(event Collision|EventActorBeginOverlap
  (params (OtherActor :type Actor%20Object%20Reference)))

(event EventTick
  (params (DeltaSeconds :type Float%20%28single-precision%29)))

(event Input|ActionEvents|InputActionFireMinigun
  (params (Key :type Key%20Structure :default "None"))
  (bind _pod (Variables|Default|GetPod))
  (:Pressed
    (Default|StartFireMinigun _pod))
  (:Released
    (Default|StopFireMinigun _pod)))

(event Input|ActionEvents|InputActionFireCanon
  (params (Key :type Key%20Structure :default "None"))
  (bind _pod (Variables|Default|GetPod))
  (:Pressed
    (Default|StartFireCanon _pod))
  (:Released
    (Default|StopFireCanon _pod)))

(fn ConstructionScript
  (|CallParentFunction))
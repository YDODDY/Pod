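; Boss enemy that patrols at random, chases a detected player and ragdolls on death, showing a health bar widget from BeginPlay.
; Detection and attack-range overlaps drive AI movement and a looping sphere-trace attack.
; BPC DamageSystem backs its health, heal and damage functions and raises death, block and response events.
; Tick re-arms a delayed block timer while switching the Block shield off every frame.
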(event OnComponentBeginOverlap(PlayerDetect)
  (params (OverlappedComponent :type Primitive%20Component%20Object%20Reference) (OtherActor :type Actor%20Object%20Reference) (OtherComp :type Primitive%20Component%20Object%20Reference) (OtherBodyIndex :type Integer) (bFromSweep :type Boolean) (SweepResult :type Hit%20Result%20Structure%20%28by%20ref%29))
  ;[1 1 1] 플레이어 감지시 플레이어 쫓아감 > 감지범위 벗어나면 배회
  (bind _asbp_player (Utilities|Casting|CastToBP_Player OtherActor))
  (Variables|Default|SetAs%20BP%20Player _asbp_player)
  (Variables|Default|SetPlayerDetected true)
  (CallFunction|MovetoPlayer)
  ;[1 1 1] 플레이어 공격반경에 있으면 Attack 실행
  (if (not (Variables|Default|GetIs%20Dead))
    (if (not (Variables|Default|GetCanAttackPlayer))
      (Utilities|Time|SetTimerbyEvent (delegate Custom|Attack) 1.0 true))))

(event OnComponentEndOverlap(PlayerDetect)
  (params (OverlappedComponent :type Primitive%20Component%20Object%20Reference) (OtherActor :type Actor%20Object%20Reference) (OtherComp :type Primitive%20Component%20Object%20Reference) (OtherBodyIndex :type Integer))
  ;[1 1 1] 플레이어 감지시 플레이어 쫓아감 > 감지범위 벗어나면 배회
  (Utilities|Casting|CastToBP_Player OtherActor)
  (Variables|Default|SetPlayerDetected false)
  (CallFunction|StopSeekingPlayer)
  (CallFunction|RandomPatrol))

(event OnComponentBeginOverlap(PlayerAttack)
  (params (OverlappedComponent :type Primitive%20Component%20Object%20Reference) (OtherActor :type Actor%20Object%20Reference) (OtherComp :type Primitive%20Component%20Object%20Reference) (OtherBodyIndex :type Integer) (bFromSweep :type Boolean) (SweepResult :type Hit%20Result%20Structure%20%28by%20ref%29))
  ;[1 1 1] 플레이어가 공격가능 범위 안에 있는지 확인
  (Utilities|Casting|CastToBP_Player OtherActor)
  (Variables|Default|SetCanAttackPlayer true))

(event OnComponentEndOverlap(PlayerAttack)
  (params (OverlappedComponent :type Primitive%20Component%20Object%20Reference) (OtherActor :type Actor%20Object%20Reference) (OtherComp :type Primitive%20Component%20Object%20Reference) (OtherBodyIndex :type Integer))
  ;[1 1 1] 플레이어가 공격가능 범위 안에 있는지 확인
  (Utilities|Casting|CastToBP_Player OtherActor)
  (Variables|Default|SetCanAttackPlayer false))

(event Custom|Random%20Patrol
  ;[1 1 1] 랜덤 돌아다님
  (AI|AIMoveTo self (.RandomLocation (AI|Navigation|GetRandomReachablePointinRadius (Transformation|GetActorLocation) 1.5e+03 0 0)) 0 5.0 false
    (:then
      (Utilities|FlowControl|Delay 1.0)
      (CallFunction|RandomPatrol))))

(event Custom|Death
  (bind _mesh (Variables|Character|GetMesh))
  ;[1 1 1] 체력 다 닳으면 죽음 > Mesh Collisionn 다 꺼버림
  (Physics|SetSimulatePhysics _mesh true)
  (Collision|SetCollisionEnabled _mesh "QueryAndPhysics")
  (Variables|Default|SetIs%20Dead true))

(event Custom|Blocked
  (params (CanBeParried :type Boolean))
  ;[1 1 1] Block 되면 Block 로그 출력
  (Development|PrintString "Blocked"))

(event Custom|DamageResponse
  (params (Damage%20Response :type E_DamageResponse%20Enum :default "NewEnumerator0"))
  ;[1 1 1] 피격시 HitResponse 로그 출력
  (Development|PrintString (Utilities|String|EnumtoString Damage%20Response)))

(event Custom|Move%20to%20Player
  ;[1 1 1] 플레이어 쫓아감
  (AI|AIMoveTo self (Transformation|GetActorLocation (Variables|Default|GetAs%20BP%20Player)) 0 5e+01 false
    (:then
      (if (Variables|Default|GetCanAttackPlayer)
        (CallFunction|StopSeekingPlayer)
        (else
          (Utilities|Time|SetTimerbyFunctionName 0 "Move to Player" 0.5 true))))))

(event Custom|Attack
  (bind _returnvalue (Transformation|GetActorForwardVector))
  ;[1 1 1] 플레이어 공격반경에 있으면 Attack 실행
  ;[1 1 1] Actor 전방으로 스피어콜리전 생성 - 닿으면 attack1
  (bind (_outhit _returnvalue_2) (Collision|SphereTraceForObjects (Transformation|GetActorLocation) (+ (- (Transformation|GetActorLocation (Variables|Default|GetAs%20BP%20Player)) _returnvalue) (* _returnvalue 1e+02)) 3e+01 (Utilities|Array|MakeArray "ObjectTypeQuery3") false 0 "ForDuration" true "(R=0.001492,G=0.000000,B=1.000000,A=1.000000)" "(R=1.000000,G=0.000000,B=0.961700,A=1.000000)" 1.0))
  (if _returnvalue_2
    (bind _wasdamaged (Class|IFDamage|TakeDamage(Message) (.HitActor (Collision|BreakHitResult _outhit)) (Utilities|Struct|MakeS_DamageInfo 1e+01 "NewEnumerator1" "NewEnumerator1")))
    (if _wasdamaged
      (Effects|SpawnEmitteratLocation "/Game/Pod/VFX/P_CanonImpact.P_CanonImpact" (.Location (Collision|BreakHitResult _outhit))))))

(event Custom|StopSeekingPlayer
  (Utilities|Time|ClearTimerbyFunctionName 0 "Move to Payer"))

(event Custom|BolckAttack
  (bind _block (Variables|Default|GetBlock))
  ;[1 1 1] 공격 방어
  (Rendering|SetVisibility _block true false)
  (Collision|SetCollisionEnabled _block "QueryAndPhysics")
  (Variables|Default|SetBlocking true))

(event Custom|EndBlockAttack
  (bind _block (Variables|Default|GetBlock))
  ;[1 1 1] 공격 방어
  (Rendering|SetVisibility _block false false)
  (Collision|SetCollisionEnabled _block "NoCollision")
  (Variables|Default|SetBlocking false))

(event EventTick
  (params (DeltaSeconds :type Float%20%28single-precision%29))
  (Utilities|Time|SetTimerbyEvent (delegate Custom|BolckAttack) 5.0)
  (CallFunction|EndBlockAttack))

(event EventBeginPlay
  (Variables|Default|SetIs%20Dead false)
  (CallFunction|RandomPatrol)
  ;[1 1 1] 화면 중앙 아래 체력바 띄움
  (bind _returnvalue (UserInterface|CreateWidget "/Game/Boss/DamageSystem/Enemy/W_BossHealth.W_BossHealth_C" 0 self))
  (UserInterface|Viewport|AddtoViewport _returnvalue 0))

(fn ConstructionScript
  (bind _bpc_damagesystem (Variables|Default|GetBPC_DamageSystem))
  ;[1 1 1] Damage System 변수 + Death, Blocked, DamageResponse
  (EventDispatchers|BindEventtoOnDeath _bpc_damagesystem (EventDispatchers|CreateEvent :!event Custom|Death))
  (EventDispatchers|BindEventtoOnBlocked _bpc_damagesystem (EventDispatchers|CreateEvent :!event Custom|Blocked))
  (EventDispatchers|BindEventtoOnDamageResponse _bpc_damagesystem (EventDispatchers|CreateEvent :!event Custom|DamageResponse)))

(fn GetCurrentHealth
  (return (Variables|/Game/Boss/DamageSystem/BPC_DamageSystem.BPC_DamageSystem_C|GetHealth (Variables|Default|GetBPC_DamageSystem))))

(fn GetMaxHealth
  (return (Variables|/Game/Boss/DamageSystem/BPC_DamageSystem.BPC_DamageSystem_C|GetMaxHealth (Variables|Default|GetBPC_DamageSystem))))

(fn Heal
  (params (Amount :type Float%20%28double-precision%29))
  (bind _newhealth (Class|IFDamage|Heal(Message) (Variables|Default|GetBPC_DamageSystem) Amount))
  (return _newhealth))

(fn TakeDamage
  (params (DamageInfo :type S%20Damage%20Info%20Structure))
  (bind _wasdamaged (Default|TakeDamage (Variables|Default|GetBPC_DamageSystem) DamageInfo))
  (return _wasdamaged))
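; BP_AutoPod is an automatic attack pod that shoots at enemies it sees.
; When its PawnSensing component spots a pawn tagged "Enermy" that casts to BP_Enemy, it turns to face that pawn.
; After a short delay, it spawns a BP_AutoPodBullet at its Arrow component's transform.
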(event OnSeePawn(PawnSensing)
  (params (Pawn :type Pawn%20Object%20Reference))
  (if (Actor|ActorHasTag Pawn "Enermy")
    (Utilities|Casting|CastToBP_Enemy Pawn)
    (Transformation|SetActorRotation (Math|Rotator|FindLookatRotation (Transformation|GetActorLocation) (Transformation|GetActorLocation Pawn)))
    (Utilities|FlowControl|Delay 0.1)
    (Game|SpawnActorfromClass "/Game/9S/9sPod/BP_AutoPodBullet.BP_AutoPodBullet_C" (Transformation|GetWorldTransform (Variables|Default|GetArrow)) "Undefined" "MultiplyWithRoot" 0 0)))

(fn ConstructionScript)
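; 9S test companion pawn that follows the player, approaches a nearby enemy and throws weapons.
; Tick refreshes player and first-found BP_CEnemy references, then starts both follow events, which re-call themselves after AI moves.
; Player distance takes priority over chasing; when the player is near, FollowPlayer targets itself.
; PawnSensing sightings of tagged enemies trigger Throwing, which spawns BP_Weapon, halts movement and briefly hides the held weapon, gated by a cooldown.
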(event OnSeePawn(PawnSensing)
  (params (Pawn :type Pawn%20Object%20Reference))
  (if (Actor|ActorHasTag Pawn "Enermy")
    (Utilities|Casting|CastToBP_C++Enemy Pawn)
    (Utilities|FlowControl|Delay 0.1)
    (CallFunction|Throwing)))

(event Custom|Follow%20Player
  ;[1 1 1] 아군따라가기
  (if (>= (Transformation|GetDistanceTo (Variables|Default|GetChar%20REF)) 1e+03)
    (AI|AIMoveTo self "0, 0, 0" (Variables|Default|GetChar%20REF) 5.0 false
      (:then
        _))
    (else
      (AI|AIMoveTo self "0, 0, 0" self 5.0 false
        (:then
          _))))
  (Utilities|FlowControl|Delay 0.1)
  (CallFunction|FollowPlayer))

(event Custom|Throwing
  ;[1 1 1] 검발사
  (if (Variables|Default|GetIs%20Throwing?)
    (Game|SpawnActorfromClass "/Game/9S/9sTest/Blueprint/BP_Weapon.BP_Weapon_C" (Math|Transform|MakeTransform (+ (Transformation|GetActorLocation) "100.000000,0.000000,0.000000") "0, 0, 0" "1.000000,1.000000,1.000000") "AlwaysSpawn" "MultiplyWithRoot" 0 0)
    (Rendering|SetVisibility (Variables|Default|Getweapon) false false)
    (Variables|Default|SetIs%20Throwing? false)
    (Components|Movement|StopMovementImmediately (Variables|Character|GetCharacterMovement))
    (Utilities|FlowControl|Delay 1.0)
    (Rendering|SetVisibility (Variables|Default|Getweapon) true false)
    (Utilities|FlowControl|Delay 2.0)
    (Variables|Default|SetIs%20Throwing? true)))

(event Custom|Follow%20Enemy
  ;[1 1 1] 에너미가 가까우면 에너미 따라, 아군이 멀어지면 아군따라가기
  (if (<= (Transformation|GetDistanceTo (Variables|Default|GetEnermy%20REF)) 8e+02)
    (if (>= (Transformation|GetDistanceTo (Variables|Default|GetChar%20REF)) 1e+03)
      (AI|AIMoveTo self "0, 0, 0" (Variables|Default|GetChar%20REF) 5.0 false
        (:then
          _))
      (else
        (AI|AIMoveTo self "0, 0, 0" (Variables|Default|GetEnermy%20REF) 5.0 false
          (:then
            _))))
    (Utilities|FlowControl|Delay 0.1)
    (CallFunction|FollowEnemy)))

(event EventTick
  (params (DeltaSeconds :type Float%20%28single-precision%29))
  ;[1 1 1] 플레이어를 따라 갈까요? 에너미를 따라갈까요?
  (Utilities|FlowControl|Sequence
    (:then_0
      (bind _asbp_player (Utilities|Casting|CastToBP_Player (Game|GetPlayerCharacter 0)))
      (Variables|Default|SetChar%20REF _asbp_player)
      (CallFunction|FollowPlayer))
    (:then_1
      (bind _returnvalue (Actor|GetActorOfClass "/Game/Boss/DamageSystem/Player/BP_C++Enemy.BP_C++Enemy_C"))
      (Variables|Default|SetEnermy%20REF _returnvalue)
      (CallFunction|FollowEnemy))))

(fn ConstructionScript)
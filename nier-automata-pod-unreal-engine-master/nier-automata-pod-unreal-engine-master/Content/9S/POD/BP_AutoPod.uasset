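; BP_AutoPod is an AI companion pod that follows the BP_9sTest character and shoots at enemies it sees.
; PawnSensing picks out BP_C++Enemy pawns tagged "Enermy", turns the pod toward them, then spawns BP_PODBULLET from its Arrow after a short delay.
; Tick looks up the character every frame and calls Follow9s, which moves toward it when distant, otherwise targets itself, and re-calls itself after a delay.
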(event OnSeePawn(PawnSensing)
  (params (Pawn :type Pawn%20Object%20Reference))
  (if (Actor|ActorHasTag Pawn "Enermy")
    (Utilities|Casting|CastToBP_C++Enemy Pawn)
    (Transformation|SetActorRotation (Math|Rotator|FindLookatRotation (Transformation|GetActorLocation) (Transformation|GetActorLocation Pawn)))
    (Utilities|FlowControl|Delay 0.1)
    (Game|SpawnActorfromClass "/Game/9S/POD/BP_PODBULLET.BP_PODBULLET_C" (Transformation|GetWorldTransform (Variables|Default|GetArrow)) "AlwaysSpawn" "MultiplyWithRoot" 0 0)
    (CallFunction|Follow9s)))

(event Custom|Follow%209s
  (if (>= (Transformation|GetDistanceTo (Variables|Default|GetChar%20Ref)) 4e+02)
    (AI|AIMoveTo self "0, 0, 0" (Variables|Default|GetChar%20Ref) 5.0 false
      (:then
        _))
    (else
      (AI|AIMoveTo self "0, 0, 0" self 5.0 false
        (:then
          _))))
  (Utilities|FlowControl|Delay 0.2)
  (CallFunction|Follow9s))

(event EventTick
  (params (DeltaSeconds :type Float%20%28single-precision%29))
  (bind _returnvalue (Actor|GetActorOfClass "/Game/9S/9sTest/Blueprint/BP_9sTest.BP_9sTest_C"))
  (Variables|Default|SetChar%20Ref _returnvalue)
  (CallFunction|Follow9s))

(fn ConstructionScript)
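; BP_9sTest is a test AI companion for 9S that follows the player and attacks enemies it sees.
; A recursive 0.1-second loop reissues AIMoveTo toward the player when at least 400 units away, otherwise targeting itself to hold position.
; PawnSensing filters for "Enermy"-tagged BP_Enemy pawns, then spawns a pod bullet from Arrow1 after a short delay.
; It then calls Throwing, which spawns BP_Weapon and hides the held weapon if IsThrowing is set.
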(event OnSeePawn(PawnSensing)
  (params (Pawn :type Pawn%20Object%20Reference))
  (if (Actor|ActorHasTag Pawn "Enermy")
    (Utilities|Casting|CastToBP_Enemy Pawn)
    (Utilities|FlowControl|Delay 0.1)
    (Game|SpawnActorfromClass "/Game/9S/9sPod/BP_PODBULLET.BP_PODBULLET_C" (Transformation|GetWorldTransform (Variables|Default|GetArrow1)) "Undefined" "MultiplyWithRoot" 0 0)
    (CallFunction|Throwing)))

(event Custom|Follow%20Player
  (if (>= (Transformation|GetDistanceTo (Variables|Default|GetChar%20REF)) 4e+02)
    (AI|AIMoveTo self "0, 0, 0" (Variables|Default|GetChar%20REF) 5.0 false
      (:then
        _))
    (else
      (AI|AIMoveTo self "0, 0, 0" self 5.0 false
        (:then
          _))))
  (Utilities|FlowControl|Delay 0.1)
  (CallFunction|FollowPlayer))

(event Custom|Throwing
  (if (Variables|Default|GetIs%20Throwing?)
    (Game|SpawnActorfromClass "/Game/9S/9sTest/Weapon/BP_Weapon.BP_Weapon_C" (Math|Transform|MakeTransform (Transformation|GetActorLocation) "0, 0, 0" "1.000000,1.000000,1.000000") "Undefined" "MultiplyWithRoot" 0 0)
    (Rendering|SetVisibility (Variables|Default|GetWeapon) false false)))

(event EventBeginPlay
  (bind _asbp_player (Utilities|Casting|CastToBP_Player (Game|GetPlayerCharacter 0)))
  (Variables|Default|SetChar%20REF _asbp_player)
  (CallFunction|FollowPlayer))

(fn ConstructionScript)